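; BP_003 is a spinning mechanism that either kills or knocks away the adventure character on contact.
; Tick rotates the Body by a fixed step each frame, independent of delta time.
; On Capsule overlap with BP_AdventureCharacter, the Death flag selects between calling Dead and applying a strong movement impulse along the Arrow's forward vector.
; The construction script shows the Thorn only when Death is set.
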(event `self.ReceiveTick`
  (params (DeltaSeconds :type "Float (single-precision)"))
  ; 【事件】事件Tick
  ; 执行链路（自动生成）：Add Relative Rotation → 获得Body
  (`SceneComponent.K2_AddRelativeRotation` (`self.Body`) (struct :`Yaw` 10.0) false false))

(event `self.Capsule.OnComponentBeginOverlap`
  (params (OverlappedComponent :type "PrimitiveComponent Object Reference") (OtherActor :type "Actor Object Reference") (OtherComp :type "PrimitiveComponent Object Reference") (OtherBodyIndex :type Integer) (bFromSweep :type Boolean) (SweepResult :type "HitResult Structure (by ref)"))
  ; 【事件】组件开始重叠时 (Capsule)
  ; 执行链路（自动生成）：类型转换为 BP_AdventureCharacter → 分支 → 变更路线节点 → 获得CharacterMovement → Dead → AddImpulse → 获得Death → vector * vector
  (bind _asbp_adventure_character (cast `/Game/Code/Character/BP_AdventureCharacter` OtherActor))
  (if (`self.Death`)
    (`/Game/Code/Character/BP_AdventureCharacter.Dead` _asbp_adventure_character)
    (else
      (`CharacterMovementComponent.AddImpulse` (`Character.CharacterMovement` _asbp_adventure_character) (* (`SceneComponent.GetForwardVector` (`self.Arrow`)) 80000) false))))

(fn `UserConstructionScript`
  (if (`self.Death`)
    (`SceneComponent.SetVisibility` (`self.Thorn`) true false)
    (else
      (`SceneComponent.SetVisibility` (`self.Thorn`) false false))))