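; Mechanism Blueprint that moves two wooden pole meshes (06 and 08) vertically, offsetting them in counter-motion from one animation track.
; BeginPlay caches both poles' relative locations, then plays a Timeline that updates their Z positions.
; Pole 06 adds the track value to its starting height, while pole 08 adds the absolute difference between that value and a fixed offset, mirroring the motion within that range.
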(event `self.ReceiveBeginPlay`
  (bind (_06location_x _06location_y _06location_z) (`KismetMathLibrary.BreakVector` (`self.06Location`)))
  (bind (_08location_x _08location_y _08location_z) (`KismetMathLibrary.BreakVector` (`self.08Location`)))
  ; 【事件】事件BeginPlay
  ; 执行链路（自动生成）：设置06Location → 设置08Location → 时间轴 → Set Relative Location → float + float → 变更路线节点 → float - float → Absolute (Float) → 获得RelativeLocation → 获得SM_WoodenPole_06 → Get → 获得SM_WoodenPole_08
  (set `self.06Location` (`SceneComponent.RelativeLocation` (`self.SM_WoodenPole_06`)))
  (set `self.08Location` (`SceneComponent.RelativeLocation` (`self.SM_WoodenPole_08`)))
  ;; 【事件】时间轴
  ;; 执行链路（自动生成）：Set Relative Location → float + float → 变更路线节点 → float - float → Absolute (Float) → 获得SM_WoodenPole_06 → Get → 获得SM_WoodenPole_08
  (bind (_direction `_新建轨道_1`) (`Timeline|时间轴`)
    (:`Update`
      (`SceneComponent.K2_SetRelativeLocation` (`self.SM_WoodenPole_06`) (`KismetMathLibrary.MakeVector` _06location_x _06location_y (+ _06location_z `_新建轨道_1`)) false false)
      (`SceneComponent.K2_SetRelativeLocation` (`self.SM_WoodenPole_08`) (`KismetMathLibrary.MakeVector` _08location_x _08location_y (+ _08location_z (`KismetMathLibrary.Abs` (- `_新建轨道_1` 150.0)))) false false))))

(fn `UserConstructionScript`)