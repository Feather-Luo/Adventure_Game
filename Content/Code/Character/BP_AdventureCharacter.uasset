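; Third-person player character for an adventure game, with Enhanced Input movement, look, jump and spring-arm camera zoom.
; BeginPlay registers IMC_Adventure; movement follows the camera's forward and right vectors, and zoom is clamped between min and max arm lengths.
; Tick calls Dead below a hardcoded height, without a guard flag.
; Dead ragdolls the mesh, disables camera collision and movement, then after a delay destroys the actor and calls Rebirth on BP_AdventureMode.
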(event `self.ReceiveBeginPlay`
  ; 【事件】BeginPlay —— 游戏/关卡开始时执行一次
  ; 作用：把增强输入映射上下文 IMC_Adventure 注册到本地玩家子系统
  ; 链路：GetPlayerController → 获取EnhancedInputLocalPlayerSubsystem → AddMappingContext
  (`EnhancedInputSubsystemInterface.AddMappingContext` (pcsubsystem `EnhancedInputLocalPlayerSubsystem` (`GameplayStatics.GetPlayerController` 0)) "/Game/Code/Character/Input/IMC_Adventure.IMC_Adventure" 0 (struct)))

(event `EnhancedInput|/Game/Code/Character/Input/IA_Move`
  (params (ActionValue :type "Vector2D Structure") (ElapsedSeconds :type "Float (double-precision)") (TriggeredSeconds :type "Float (double-precision)") (InputAction :type "InputAction Object Reference" :default "/Game/Code/Character/Input/IA_Move.IA_Move"))
  (bind (_x _y) (`KismetMathLibrary.BreakVector2D` ActionValue))
  (bind _camera (`self.Camera`))
  ; 【事件】IA_Move —— 移动输入（W / A / S / D）
  ; 作用：把 Axis2D 输入值拆成 X、Y 两个分量，分别乘以相机的「前向向量」和「右向向量」，
  ; 　　　再交给 AddMovementInput 驱动角色移动（所以移动方向跟随相机朝向）
  ; 链路：ActionValue → BreakVector2D → (× GetForwardVector / × GetRightVector) → AddMovementInput ×2
  (:`Triggered`
    (`self.AddMovementInput` (`SceneComponent.GetForwardVector` _camera) _x)
    (`self.AddMovementInput` (`SceneComponent.GetRightVector` _camera) _y)))

(event `EnhancedInput|/Game/Code/Character/Input/IA_Look`
  (params (ActionValue :type "Vector2D Structure") (ElapsedSeconds :type "Float (double-precision)") (TriggeredSeconds :type "Float (double-precision)") (InputAction :type "InputAction Object Reference" :default "/Game/Code/Character/Input/IA_Look.IA_Look"))
  (bind (_x _y) (`KismetMathLibrary.BreakVector2D` ActionValue))
  ; 【事件】IA_Look —— 视角输入（鼠标移动）
  ; 作用：Axis2D 的 X 分量驱动控制器 Yaw（左右转视角），Y 分量驱动 Pitch（上下看）
  ; 链路：ActionValue → BreakVector2D → AddControllerYawInput / AddControllerPitchInput
  (:`Triggered`
    (`self.AddControllerYawInput` _x)
    (`self.AddControllerPitchInput` _y)))

(event `EnhancedInput|/Game/Code/Character/Input/IA_Jump`
  (params (ActionValue :type Boolean) (ElapsedSeconds :type "Float (double-precision)") (TriggeredSeconds :type "Float (double-precision)") (InputAction :type "InputAction Object Reference" :default "/Game/Code/Character/Input/IA_Jump.IA_Jump"))
  ; 【事件】IA_Jump —— 跳跃输入（空格）
  ; 作用：调用角色自带的 Jump
  ; 链路：Triggered → Jump
  (:`Started`
    (`self.Jump`)))

(event `EnhancedInput|/Game/Code/Character/Input/IA_CameraZoom`
  (params (ActionValue :type "Float (double-precision)") (ElapsedSeconds :type "Float (double-precision)") (TriggeredSeconds :type "Float (double-precision)") (InputAction :type "InputAction Object Reference" :default "/Game/Code/Character/Input/IA_CameraZoom.IA_CameraZoom"))
  (bind _springarm (`self.SpringArm`))
  ; 【事件】IA_CameraZoom —— 鼠标滚轮缩放第三人称视角
  ; 作用：滚轮上滚拉近、下滚拉远，并限制在 [MinArmLength, MaxArmLength] 区间
  ; 公式：新臂长 = Clamp(当前臂长 − 滚轮值 × ZoomStep, MinArmLength, MaxArmLength)
  ; 链路：ActionValue(双击) × ZoomStep(双击) → Subtract(当前臂长 − 步长)
  ; 　　　→ Clamp(Min, Max) → SpringArm 的 Set Target Arm Length
  ; 说明：ActionValue 对 Axis1D 动作本身就是 double 引脚，无需转换节点；
  ; 　　　用「减法」让滚轮正向=拉近，无需 Negate 修饰器
  (:`Triggered`
    (set `SpringArmComponent.TargetArmLength` (`KismetMathLibrary.FClamp` (- (`SpringArmComponent.TargetArmLength` _springarm) (* ActionValue (`self.ZoomStep`))) (`self.MinArmLength`) (`self.MaxArmLength`)) _springarm)))

(event `Dead`
  ; 【自定义事件】Dead —— 角色死亡处理
  ; 步骤：① 骨架网格开启物理模拟（Ragdoll 倒地）
  ; 　　　② 弹簧臂关闭碰撞检测（防止尸体抖动）
  ; 　　　③ 移动模式设为 None（停止一切移动）
  ; 　　　④ 延时后销毁角色本体 Destroy Actor
  ; 　　　⑤ 通过 GameMode → Rebirth 触发重生
  ; 链路：获得Mesh → SetSimulatePhysics / 设置bDoCollisionTest=False / SetMovementMode(None)
  ; 　　　→ Delay → Destroy Actor → GetGameMode → 类型转换为BP_AdventureMode → Rebirth
  (`PrimitiveComponent.SetSimulatePhysics` (`self.Mesh`) true)
  (set `SpringArmComponent.bDoCollisionTest` false (`self.SpringArm`))
  (`CharacterMovementComponent.SetMovementMode` (`self.CharacterMovement`) "MOVE_None" 0)
  (`KismetSystemLibrary.Delay` 2.0)
  (`self.K2_DestroyActor`)
  (bind _asbp_adventure_mode (cast `/Game/Code/Character/BP_AdventureMode` (`GameplayStatics.GetGameMode`)))
  (`/Game/Code/Character/BP_AdventureMode.Rebirth` _asbp_adventure_mode))

(event `self.ReceiveTick`
  (params (DeltaSeconds :type "Float (single-precision)"))
  (bind (_returnvalue_x _returnvalue_y _returnvalue_z) (`KismetMathLibrary.BreakVector` (`self.K2_GetActorLocation`)))
  ; 【事件】Tick —— 每帧执行一次
  ; 作用：掉落死亡判定。取角色世界坐标 Z，与阈值比较（float <= float），
  ; 　　　若低于阈值则走「分支」的 True 分支调用 Dead 事件
  ; 链路：Get Actor Location → (Z <= 阈值) → 分支 → Dead
  (if (<= _returnvalue_z 460.0)
    (`self.Dead`)))

(fn `UserConstructionScript`)